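; Player Blueprint that creates the main interface widget on BeginPlay and adds it to the viewport.
; The I key alternates the interface between its inventory and crosshair views through a FlipFlop.
; An AddItemtoInventoryWidget event wraps incoming item data in an inventory item widget and adds it to the interface's inventory panel.
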(event `self.ReceiveBeginPlay`
  (bind _returnvalue (`|CreateWidget` "/Game/Widgets/W_Interface.W_Interface_C"))
  (set `self.W_UI` _returnvalue)
  (`UserWidget.AddToViewport` _returnvalue 0))

(event `Key|I`
  (params (Key :type "Key Structure"))
  (bind _w_ui (`self.W_UI`))
  (:`Pressed`
    (`/Engine/EditorBlueprintResources/StandardMacros.FlipFlop`
      (:`A`
        (`/Game/Widgets/W_Interface.Inventory` _w_ui))
      (:`B`
        (`/Game/Widgets/W_Interface.CrossHair` _w_ui)))))

(event `self.AddItemToInventoryWidget`
  (params (ItemData :type "Item_Information Structure"))
  (bind _returnvalue (`|CreateWidget` "/Game/Widgets/W_InventoryItem.W_InventoryItem_C" null ItemData))
  (`/Game/Widgets/W_Inventory.AddItem` (`/Game/Widgets/W_Interface.W_Inventory` (`self.W_UI`)) _returnvalue))

(fn `UserConstructionScript`)